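; BP_NPS_AI is an AI controller for guard NPCs that tracks sensed targets for a behavior tree.
; On BeginPlay it sets up the PatrolData blackboard, runs GuardBehavior and caches the blackboard component.
; AI perception updates write sensed actors lacking the "Enemy" tag to the enemy key and clear it when such an actor is lost.
; Both perception outcomes print debug strings.
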(event `self.ReceiveBeginPlay`
  (bind _blackboardcomponent (`self.UseBlackboard` "/Game/Dynamic/NPS/AI/PatrolData.PatrolData"))
  (`self.RunBehaviorTree` "/Game/Dynamic/NPS/AI/GuardBehavior.GuardBehavior")
  (set `self.BlackBordComp` _blackboardcomponent))

(event `self.AIPerception.OnTargetPerceptionUpdated`
  (params (Actor :type "Actor Object Reference") (Stimulus :type "AIStimulus Structure"))
  (bind _blackbordcomp (`self.BlackBordComp`))
  (if (`self.ActorHasTag` Actor "Enemy")
    _
    (elif (`.bSuccessfullySensed` (break `AIStimulus` Stimulus))
      (`BlackboardComponent.SetValueAsObject` _blackbordcomp (`self.EnemyKey`) Actor)
      (`KismetSystemLibrary.PrintString` (`KismetSystemLibrary.GetDisplayName` _blackbordcomp))
      (else
        (`BlackboardComponent.ClearValue` (`self.BlackBordComp`) (`self.EnemyKey`))
        (`KismetSystemLibrary.PrintString` "Clear")))))

(fn `UserConstructionScript`)